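; BP_Monster1 is a monster that can spit at the player and is destroyed on contact with the player in a certain state.
; Fire snaps the monster to face the player character, then spawns BP_Spit at the ShotPos transform.
; A capsule hit from the controlled pawn destroys the monster if BP_PaperCharacter's IsGgogit flag is set.
; SetMode stores a mode and switches on it with empty branches; nothing here calls it or Fire.
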(event `self.CapsuleComponent.OnComponentHit`
  (params (HitComponent :type "PrimitiveComponent Object Reference") (OtherActor :type "Actor Object Reference") (OtherComp :type "PrimitiveComponent Object Reference") (NormalImpulse :type "Vector Structure") (Hit :type "HitResult Structure (by ref)"))
  (if (== OtherActor (`Controller.K2_GetPawn` (`GameplayStatics.GetPlayerController` 0)))
    (bind _returnvalue (`GameplayStatics.GetActorOfClass` "/Game/03_Blueprints/BP_PaperCharacter.BP_PaperCharacter_C"))
    (if (`/Game/03_Blueprints/BP_PaperCharacter.isGgogit` _returnvalue)
      (`self.K2_DestroyActor`))))

(fn `Fire`
  (`self.K2_SetActorRotation` (`KismetMathLibrary.FindLookAtRotation` (`self.K2_GetActorLocation`) (`self.K2_GetActorLocation` (`GameplayStatics.GetPlayerCharacter` 0))))
  (`|SpawnActorFromClass` "/Game/Monster/BP_Spit.BP_Spit_C" (`SceneComponent.K2_GetComponentToWorld` (`self.ShotPos`)) "Undefined" "OverrideRootScale" null null))

(fn `SetMode`
  (params (mode :type Integer))
  (bind _output_get (set `self.mode` mode))
  (switch `int` _output_get))

(fn `UserConstructionScript`)