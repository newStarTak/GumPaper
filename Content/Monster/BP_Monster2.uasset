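; BP_Monster2 is a monster that shoots spray projectiles and can be destroyed by contact with the player.
; Fire turns it toward the player with pitch zeroed and spawns BP_Spray actors at eight shot points.
; A capsule hit by the player's pawn destroys the monster after a three-second delay, unless Gum_BP is in balloon state.
; SetMode stores a mode but its switch has no behavior, and nothing here calls Fire.
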(event `self.CapsuleComponent.OnComponentHit`
  (params (HitComponent :type "PrimitiveComponent Object Reference") (OtherActor :type "Actor Object Reference") (OtherComp :type "PrimitiveComponent Object Reference") (NormalImpulse :type "Vector Structure") (Hit :type "HitResult Structure (by ref)"))
  (bind _returnvalue (== OtherActor (`Controller.K2_GetPawn` (`GameplayStatics.GetPlayerController` 0))))
  (if _returnvalue
    (`KismetSystemLibrary.Delay` 3.0)
    (if _returnvalue
      (bind _returnvalue_2 (`GameplayStatics.GetActorOfClass` "/Game/03_Blueprints/Gum_BP.Gum_BP_C"))
      (if (not (`/Game/03_Blueprints/Gum_BP.isBalloon` _returnvalue_2))
        (`self.K2_DestroyActor`)))))

(fn `Fire`
  (bind (_returnvalue_roll _returnvalue_pitch _returnvalue_yaw) (`KismetMathLibrary.BreakRotator` (`KismetMathLibrary.FindLookAtRotation` (`self.K2_GetActorLocation`) (`self.K2_GetActorLocation` (`GameplayStatics.GetPlayerCharacter` 0)))))
  (`self.K2_SetActorRotation` (`KismetMathLibrary.MakeRotator` _returnvalue_roll 0.0 _returnvalue_yaw))
  (`|SpawnActorFromClass` "/Game/Monster/BP_Spray.BP_Spray_C" (`SceneComponent.K2_GetComponentToWorld` (`self.ShotPos1`)) "Undefined" "OverrideRootScale" null null)
  (`|SpawnActorFromClass` "/Game/Monster/BP_Spray.BP_Spray_C" (`SceneComponent.K2_GetComponentToWorld` (`self.ShotPos2`)) "Undefined" "OverrideRootScale" null null)
  (`|SpawnActorFromClass` "/Game/Monster/BP_Spray.BP_Spray_C" (`SceneComponent.K2_GetComponentToWorld` (`self.ShotPos3`)) "Undefined" "OverrideRootScale" null null)
  (`|SpawnActorFromClass` "/Game/Monster/BP_Spray.BP_Spray_C" (`SceneComponent.K2_GetComponentToWorld` (`self.ShotPos4`)) "Undefined" "OverrideRootScale" null null)
  (`|SpawnActorFromClass` "/Game/Monster/BP_Spray.BP_Spray_C" (`SceneComponent.K2_GetComponentToWorld` (`self.ShotPos5`)) "Undefined" "OverrideRootScale" null null)
  (`|SpawnActorFromClass` "/Game/Monster/BP_Spray.BP_Spray_C" (`SceneComponent.K2_GetComponentToWorld` (`self.ShotPos6`)) "Undefined" "OverrideRootScale" null null)
  (`|SpawnActorFromClass` "/Game/Monster/BP_Spray.BP_Spray_C" (`SceneComponent.K2_GetComponentToWorld` (`self.ShotPos9`)) "Undefined" "OverrideRootScale" null null)
  (`|SpawnActorFromClass` "/Game/Monster/BP_Spray.BP_Spray_C" (`SceneComponent.K2_GetComponentToWorld` (`self.ShotPos8`)) "Undefined" "OverrideRootScale" null null))

(fn `SetMode`
  (params (mode :type Integer))
  (bind _output_get (set `self.mode` mode))
  (switch `int` _output_get))

(fn `UserConstructionScript`)