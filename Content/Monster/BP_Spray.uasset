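; BP_Spray is a moving actor that refills gum HP when the player touches it and kills BP_Monster3 on contact.
; Tick pushes it along local X by Speed without sweep.
; Its SphereCollision overlap with the player pawn destroys the spray and sets GumHp on the first Gum_BP to full 100.
; Other overlaps destroy only the BP_Monster3 instance returned by GetActorOfClass, leaving the spray alive.
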(event `self.ReceiveTick`
  (params (DeltaSeconds :type "Float (single-precision)"))
  (`self.K2_AddActorLocalOffset` (`KismetMathLibrary.MakeVector` (* DeltaSeconds (`self.speed`)))))

(event `self.SphereCollision.OnComponentBeginOverlap`
  (params (OverlappedComponent :type "PrimitiveComponent Object Reference") (OtherActor :type "Actor Object Reference") (OtherComp :type "PrimitiveComponent Object Reference") (OtherBodyIndex :type Integer) (bFromSweep :type Boolean) (SweepResult :type "HitResult Structure (by ref)"))
  (if (== OtherActor (`Controller.K2_GetPawn` (`GameplayStatics.GetPlayerController` 0)))
    (`self.K2_DestroyActor`)
    (bind _returnvalue (`GameplayStatics.GetActorOfClass` "/Game/03_Blueprints/Gum_BP.Gum_BP_C"))
    (set `/Game/03_Blueprints/Gum_BP.GumHp` 100.0 _returnvalue)
    (`KismetSystemLibrary.PrintText` "GumHP+")
    (else
      (bind _returnvalue_2 (`GameplayStatics.GetActorOfClass` "/Game/Monster/BP_Monster3.BP_Monster3_C"))
      (if (== OtherActor _returnvalue_2)
        (`self.K2_DestroyActor` _returnvalue_2)))))

(fn `UserConstructionScript`)