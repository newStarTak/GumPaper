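; AI controller for BP_Monster1 that runs the BT_AI1 behavior tree and supplies its blackboard.
; On BeginPlay it copies the locations of the monster's two patrol point actors into the blackboard.
; Perception updates pass actors to CheckPlayerActor, which toggles PlayerActorKey for "Player"-tagged actors: it sets the key when empty and clears it otherwise, without reading whether the stimulus was sensed or lost.
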(event `self.ReceiveBeginPlay`
  (`self.RunBehaviorTree` "/Game/Monster/BT_AI1.BT_AI1")
  (`self.InitPatrolPoint`))

(event `self.AIPerception.OnPerceptionUpdated`
  (params (UpdatedActors :type "Array of Actor Object Reference (by ref)"))
  (for _array_element UpdatedActors
    (`self.CheckPlayerActor` _array_element)))

(fn `CheckPlayerActor`
  (params (SensedActor :type "Actor Object Reference"))
  (if (`self.ActorHasTag` SensedActor "Player")
    (`/Engine/EditorBlueprintResources/StandardMacros.IsValid` (`BlackboardComponent.GetValueAsObject` (`AIBlueprintHelperLibrary.GetBlackboard` null) "PlayerActorKey")
      (:`Is Valid`
        (`BlackboardComponent.SetValueAsObject` (`AIBlueprintHelperLibrary.GetBlackboard` null) "PlayerActorKey" null))
      (:`Is Not Valid`
        (`BlackboardComponent.SetValueAsObject` (`AIBlueprintHelperLibrary.GetBlackboard` null) "PlayerActorKey" SensedActor)))))

(fn `InitPatrolPoint`
  (bind _asbp_monster_1 (cast `/Game/Monster/BP_Monster1` (`self.K2_GetPawn`)))
  (`BlackboardComponent.SetValueAsVector` (`AIBlueprintHelperLibrary.GetBlackboard` null) "PatrolPoint1" (`self.K2_GetActorLocation` (`/Game/Monster/BP_Monster1.PatrolPoint1` _asbp_monster_1)))
  (`BlackboardComponent.SetValueAsVector` (`AIBlueprintHelperLibrary.GetBlackboard` null) "PatrolPoint2" (`self.K2_GetActorLocation` (`/Game/Monster/BP_Monster1.PatrolPoint2` _asbp_monster_1))))

(fn `UserConstructionScript`)