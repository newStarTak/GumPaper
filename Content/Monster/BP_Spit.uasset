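; BP_Spit is a monster projectile that flies straight along its local forward axis and damages the player on contact.
; Tick moves it each frame by Speed scaled with delta time, without sweeping.
; When its sphere collision overlaps the player's pawn, it destroys itself, calls WaterDamage on the first BP_PaperCharacter found in the level and prints a hit message.
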(event `self.ReceiveTick`
  (params (DeltaSeconds :type "Float (single-precision)"))
  (`self.K2_AddActorLocalOffset` (`KismetMathLibrary.MakeVector` (* DeltaSeconds (`self.speed`)))))

(event `self.SphereCollision.OnComponentBeginOverlap`
  (params (OverlappedComponent :type "PrimitiveComponent Object Reference") (OtherActor :type "Actor Object Reference") (OtherComp :type "PrimitiveComponent Object Reference") (OtherBodyIndex :type Integer) (bFromSweep :type Boolean) (SweepResult :type "HitResult Structure (by ref)"))
  (if (== OtherActor (`Controller.K2_GetPawn` (`GameplayStatics.GetPlayerController` 0)))
    (`self.K2_DestroyActor`)
    (bind _returnvalue (`GameplayStatics.GetActorOfClass` "/Game/03_Blueprints/BP_PaperCharacter.BP_PaperCharacter_C"))
    (`/Game/03_Blueprints/BP_PaperCharacter.waterDamage` _returnvalue)
    (`KismetSystemLibrary.PrintText` "Hit_HP-")))

(fn `UserConstructionScript`)