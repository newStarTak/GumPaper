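; BP_Monster3 is a monster with a walk-speed-driven movement component that damages the gum when it collides with the player.
; A capsule hit against the player's pawn finds the Gum_BP actor by class, lowers its GumHp by a small fixed amount and prints the result.
; SpeedToSlow and SpeedToFast halve and double the current max walk speed.
; SetMode stores the mode, but its switch has no branch logic.
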(event `self.CapsuleComponent.OnComponentHit`
  (params (HitComponent :type "PrimitiveComponent Object Reference") (OtherActor :type "Actor Object Reference") (OtherComp :type "PrimitiveComponent Object Reference") (NormalImpulse :type "Vector Structure") (Hit :type "HitResult Structure (by ref)"))
  (if (== OtherActor (`Controller.K2_GetPawn` (`GameplayStatics.GetPlayerController` 0)))
    (bind _returnvalue (`GameplayStatics.GetActorOfClass` "/Game/03_Blueprints/Gum_BP.Gum_BP_C"))
    (bind _gumhp (`/Game/03_Blueprints/Gum_BP.GumHp` _returnvalue))
    (set `/Game/03_Blueprints/Gum_BP.GumHp` (- _gumhp 0.05) _returnvalue)
    (`KismetSystemLibrary.PrintText` (`KismetTextLibrary.Conv_DoubleToText` _gumhp "HalfToEven"))))

(fn `SetMode`
  (params (mode :type Integer))
  (bind _output_get (set `self.mode` mode))
  (switch `int` _output_get))

(fn `SpeedToFast`
  (bind _charactermovement (`self.CharacterMovement`))
  (set `CharacterMovementComponent.MaxWalkSpeed` (* (`CharacterMovementComponent.MaxWalkSpeed` _charactermovement) 2.0) _charactermovement))

(fn `SpeedToSlow`
  (bind _charactermovement (`self.CharacterMovement`))
  (set `CharacterMovementComponent.MaxWalkSpeed` (* (`CharacterMovementComponent.MaxWalkSpeed` _charactermovement) 0.5) _charactermovement))

(fn `UserConstructionScript`)