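; Compressor hazard actor that slams up and down and affects the player paper character when it overlaps them.
; On overlap with the player's pawn, it casts to BP_PaperCharacter and sets PaperHp to 100, which the comments describe as fully charging the gauge.
; Tick runs through chained Delays to repeatedly offset the actor down and back up in instant, unswept jumps.
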(event `self.ReceiveActorBeginOverlap`
  (params (OtherActor :type "Actor Object Reference"))
  ;[1 1 1] if 플레이어가 압축기에 깔리면 (정확히는 압축기의 압축 면에 닿으면)
  (if (== OtherActor (`Controller.K2_GetPawn` (`GameplayStatics.GetPlayerController` 0)))
    ;[1 1 1] 현재는 깔렸다! 라고 출력되기만 함
    ; 반듯 게이지 모두 충전되도록 변경
    (bind _asbp_paper_character (cast `/Game/03_Blueprints/BP_PaperCharacter` (`GameplayStatics.GetPlayerPawn` 0)))
    (bind _output_get (set `self.paperVar` _asbp_paper_character))
    (set `/Game/03_Blueprints/BP_PaperCharacter.paperHp` 100.0 _output_get)))

(event `self.ReceiveTick`
  (params (DeltaSeconds :type "Float (single-precision)"))
  ;[1 1 1] 압축기 위아래 이동 무한반복
  (`KismetSystemLibrary.Delay` 2.0)
  (`self.K2_AddActorLocalOffset` (0.0 0.0 -500.0))
  (`KismetSystemLibrary.Delay` 1.0)
  (`self.K2_AddActorLocalOffset` (0.0 0.0 500.0)))

(fn `UserConstructionScript`)