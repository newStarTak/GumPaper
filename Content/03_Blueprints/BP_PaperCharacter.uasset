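; Player paper character that shapeshifts between basic, crumpled-ball and airplane forms while its paper HP drains.
; Tick drains HP, updates the widget gauge, flags crumpled state at low HP, and only prints GameOver at zero.
; ChangeMode toggles ball when crumpled, otherwise airplane with a boosting jump; landing or delayed low-HP check reverts airplane.
; Transform functions swap mesh visibility, capsule size, speed and gravity; airplane also raises drain, and WaterDamage subtracts HP.
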(event `self.ReceiveTick`
  (params (DeltaSeconds :type "Float (single-precision)"))
  ;[1 1 1] 게이지 업데이트
  (set `self.paperHp` (- (`self.paperHp`) (* (`self.damage`) DeltaSeconds)))
  (set `/Game/03_Blueprints/paperHp_BP.hpValuePercent` (/ (`self.paperHp`) (`self.paperHpInit`)) (`self.paperHp_UI`))
  ;[1 1 1] 게이지 상태 체크
  (set `self.isGgogit` (<= (`self.paperHp`) 50.0))
  ;[1 1 1] 비행 중 꼬깃상태 변환 (3초 생각보다 길지도?)
  (if (and (`self.isGgogit`) (`self.isAirplane`))
    (`KismetSystemLibrary.Delay` 3.0)
    (`self.airplaneToBasic`))
  ;[1 1 1] 게이지가 0이 되어 게임 오버
  (if (<= (`self.paperHp`) 0.0)
    (`KismetSystemLibrary.PrintString` "GameOver")))

(event `self.ReceiveBeginPlay`
  ;[1 1 1] paperHp widget에 접근
  (bind _aspaper_hp_bp (cast `/Game/03_Blueprints/paperHp_BP` (`WidgetComponent.GetUserWidgetObject` (`self.hpWidget`))))
  (bind _output_get (set `self.paperHp_UI` _aspaper_hp_bp))
  ;[1 1 1] 게이지 초기화
  (set `/Game/03_Blueprints/paperHp_BP.hpValuePercent` (/ (`self.paperHp`) (`self.paperHpInit`)) _output_get)
  (`UserWidget.AddToViewport` (`self.paperHp_UI`) 0))

(event `InputAction|ChangeMode`
  (params (Key :type "Key Structure"))
  ;[1 1 1] 상태에 따라 다르게 변신
  (:`Pressed`
    (if (`self.isGgogit`)
      ;[1 1 1] 기본 / 꼬깃 변신
      (if (`self.isBall`)
        (`self. ggogitToBasic`)
        (else
          (`self.basicToGgogit`)))
      (else
        ;[1 1 1] 기본 / 비행기 변신
        (if (`self.isAirplane`)
          (`self.airplaneToBasic`)
          (else
            (`self.basicToAirplane`)
            ;[1 1 1] 순간 상승
            (set `self.JumpMaxHoldTime` 1.0)
            (`self.Jump`)))))))

(event `self.OnLanded`
  (params (Hit :type "HitResult Structure (by ref)"))
  ;[1 1 1] 땅에 닿으면 비행기 모드 해제
  (if (`self.isAirplane`)
    (set `self.JumpMaxHoldTime` 0.0)
    (`self.airplaneToBasic`)))

(fn ` ggogitToBasic`
  (bind _charactermovement (`self.CharacterMovement`))
  ;[1 1 1] 꼬깃 -> 기본 모양 변환
  (`SceneComponent.SetHiddenInGame` (`self.Mesh`) false false)
  (`SceneComponent.SetHiddenInGame` (`self.GgogitMesh`) true false)
  (`CapsuleComponent.SetCapsuleSize` (`self.CapsuleComponent`) 42.0 96.0 true)
  ;[1 1 1] 속도 복구
  (set `CharacterMovementComponent.MaxWalkSpeed` (* (`CharacterMovementComponent.MaxWalkSpeed` _charactermovement) 0.5) _charactermovement)
  ;[1 1 1] 점프력 복구
  (set `CharacterMovementComponent.GravityScale` 1.0 (`self.CharacterMovement`))
  (set `self.isBall` false)
  (set `self.isMode` false))

(fn `airplaneToBasic`
  (bind _charactermovement (`self.CharacterMovement`))
  ;[1 1 1] 비행기 -> 기본 모양 변환
  (`SceneComponent.SetHiddenInGame` (`self.Mesh`) false false)
  (`SceneComponent.SetHiddenInGame` (`self.AirplaneMesh`) true false)
  (`CapsuleComponent.SetCapsuleSize` (`self.CapsuleComponent`) 42.0 96.0 true)
  (set `self.damage` 0.5)
  ;[1 1 1] 속도 복구
  (set `CharacterMovementComponent.MaxFlySpeed` (* (`CharacterMovementComponent.MaxFlySpeed` _charactermovement) 0.5) _charactermovement)
  ;[1 1 1] 중력 복구
  (set `CharacterMovementComponent.GravityScale` 1.0 (`self.CharacterMovement`))
  (set `self.isAirplane` false)
  (set `self.isMode` false))

(fn `basicToAirplane`
  (bind _charactermovement (`self.CharacterMovement`))
  ;[1 1 1] 기본 -> 비행기 모양 변환
  (`SceneComponent.SetHiddenInGame` (`self.Mesh`) true false)
  (`SceneComponent.SetHiddenInGame` (`self.AirplaneMesh`) false false)
  (`CapsuleComponent.SetCapsuleSize` (`self.CapsuleComponent`) 30.0 20.0 true)
  (set `self.damage` 1.0)
  ;[1 1 1] 속도 증가 (2배)
  (set `CharacterMovementComponent.MaxFlySpeed` (* (`CharacterMovementComponent.MaxFlySpeed` _charactermovement) 2.0) _charactermovement)
  ;[1 1 1] 중력 절반
  (set `CharacterMovementComponent.GravityScale` 0.5 (`self.CharacterMovement`))
  (set `self.isAirplane` true)
  (set `self.isMode` true))

(fn `basicToGgogit`
  (bind _charactermovement (`self.CharacterMovement`))
  ;[1 1 1] 기본 -> 꼬깃 모양 변환
  (`SceneComponent.SetHiddenInGame` (`self.Mesh`) true false)
  (`SceneComponent.SetHiddenInGame` (`self.GgogitMesh`) false false)
  (`CapsuleComponent.SetCapsuleSize` (`self.CapsuleComponent`) 30.0 20.0 true)
  ;[1 1 1] 속도 증가 (2배)
  (set `CharacterMovementComponent.MaxWalkSpeed` (* (`CharacterMovementComponent.MaxWalkSpeed` _charactermovement) 2.0) _charactermovement)
  ;[1 1 1] 점프력 저하 (중력 * 2)
  (set `CharacterMovementComponent.GravityScale` 2.0 (`self.CharacterMovement`))
  (set `self.isBall` true)
  (set `self.isMode` true))

(fn `UserConstructionScript`
  (`SceneComponent.SetHiddenInGame` (`self.GgogitMesh`) true false)
  (`SceneComponent.SetHiddenInGame` (`self.AirplaneMesh`) true false)
  (`self.K2_SetActorLocation` (0.0 0.0 0.0)))

(fn `waterDamage`
  (set `self.paperHp` (- (`self.paperHp`) 5.0)))