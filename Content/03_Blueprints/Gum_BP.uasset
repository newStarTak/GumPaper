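; Gum character Blueprint that transforms between a basic gum body and a slower, low-gravity bubblegum balloon form.
; ChangeMode input is blocked when tired (HP at most 25, checked only at BeginPlay); transform functions swap meshes, capsule size, speed and gravity.
; IsBalloon is cleared before its branch, so every press runs BasicToBalloon, halving speed again.
; Holding Space raises the actor each Tick in either form.
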(event `self.ReceiveBeginPlay`
  ;[1 1 1] 게이지 상태 체크
  (set `self.isTired` (<= (`self.GumHp`) 25.0)))

(event `InputAction|ChangeMode`
  (params (Key :type "Key Structure"))
  ;[1 1 1] 상태에 따라 다르게 변신
  (:`Pressed`
    (if (`self.isTired`)
      (`KismetSystemLibrary.PrintString` "25%이하 변신x")
      (else
        (bind _output_get (set `self.isBalloon` false))
        (if _output_get
          (`self.balloonToBasic`)
          (set `self.isBalloon` true)
          (else
            (`self.basicToBalloon`)
            (set `self.isBalloon` false)))))))

(event `self.ReceiveTick`
  (params (DeltaSeconds :type "Float (single-precision)"))
  ;[1 1 1] 풍선껌 상태에서 공중 활공(isballoon 이 작동하지 않아 일반껌 상태에서도 작동하니 추후 수정 바람)
  (if (`PlayerController.IsInputKeyDown` (`GameplayStatics.GetPlayerController` 0) "SpaceBar")
    (`self.K2_AddActorLocalOffset` (0.0 0.0 10.0))))

(fn `balloonToBasic`
  (bind _charactermovement (`self.CharacterMovement`))
  ;[1 1 1] 풍선껌 -> 기본 모양 변환
  (`SceneComponent.SetHiddenInGame` (`self.Mesh`) false false)
  (`SceneComponent.SetHiddenInGame` (`self.BalloonMesh`) true false)
  (`CapsuleComponent.SetCapsuleSize` (`self.CapsuleComponent`) 42.0 96.0 true)
  ;[1 1 1] 속도 복구
  (set `CharacterMovementComponent.MaxWalkSpeed` (* (`CharacterMovementComponent.MaxWalkSpeed` _charactermovement) 2.0) _charactermovement)
  ;[1 1 1] 중력 복구
  (set `CharacterMovementComponent.GravityScale` 1.0 (`self.CharacterMovement`)))

(fn `basicToBalloon`
  (bind _charactermovement (`self.CharacterMovement`))
  ;[1 1 1] 기본 -> 풍선껌 모양 변환
  (`SceneComponent.SetHiddenInGame` (`self.Mesh`) true false)
  (`SceneComponent.SetHiddenInGame` (`self.BalloonMesh`) false false)
  (`CapsuleComponent.SetCapsuleSize` (`self.CapsuleComponent`) 30.0 20.0 true)
  ;[1 1 1] 속도 감소 (0.5배)
  (set `CharacterMovementComponent.MaxWalkSpeed` (* (`CharacterMovementComponent.MaxWalkSpeed` _charactermovement) 0.5) _charactermovement)
  ;[1 1 1] 중력 영향 감소
  (set `CharacterMovementComponent.GravityScale` 0.2 (`self.CharacterMovement`)))

(fn `UserConstructionScript`
  (`SceneComponent.SetHiddenInGame` (`self.BalloonMesh`) true false))