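; Firewood pickup actor that the player collects by walking into its overlap area.
; On begin overlap it checks for player 0's controlled pawn, casts it to Gum_BP and increments that pawn's GetWood count.
; It then destroys itself, with debug prints for the pickup message and new count.
; Interact-key pickup and an overhead wood counter are noted as unfinished work.
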(event `self.ReceiveActorBeginOverlap`
  (params (OtherActor :type "Actor Object Reference"))
  (bind _returnvalue (`Controller.K2_GetPawn` (`GameplayStatics.GetPlayerController` 0)))
  ;[1 1 1] if 플레이어가 장작 근처에 있으면 (정확히는 장작보다 큰 박스 트리거 안에 있으면)
  (if (== OtherActor _returnvalue)
    ;[1 1 1] 캐릭터 개발자(이가현)가 손봐야 할 곳.
    ; 현재는 장작 근처로 가면 장작을 획득했다! 라고 하고 장작이 사라질 뿐이다.
    ; 상호작용 키 누를 시 장작은 사라져 획득 처리되고 플레이어 머리 위에 장작을 몇개 가졌는지 표시해줘야 한다.
    (`KismetSystemLibrary.PrintString` "장작을 획득했다!")
    (bind _asgum_bp (cast `/Game/03_Blueprints/Gum_BP` _returnvalue))
    (set `/Game/03_Blueprints/Gum_BP.getWood` (+ (`/Game/03_Blueprints/Gum_BP.getWood` _asgum_bp) 1) _asgum_bp)
    ;[1 1 1] test print
    (`KismetSystemLibrary.PrintString` (`KismetStringLibrary.Conv_IntToString` (`/Game/03_Blueprints/Gum_BP.getWood` _asgum_bp)))
    (`self.K2_DestroyActor`)))

(fn `UserConstructionScript`)